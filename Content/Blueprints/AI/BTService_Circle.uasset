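; Behavior tree service that makes an AI pawn circle-strafe around its target actor while keeping focus on it.
; Each tick it writes a TargetLocation to the blackboard, offset from the pawn by Distance along the cross product of the direction to target and up.
; Activation picks a random side, and a nonzero ChangeDirectionRange starts a self-rearming random timer that flips it.
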(event Custom|OnDirectionChange
  (bind _changedirectionrange (Variables|Default|GetChangeDirectionRange))
  (Variables|Default|SetFlipDirection (not (Variables|Default|GetFlipDirection)))
  (Utilities|Time|SetTimerbyEvent (delegate Custom|OnDirectionChange) (Math|Random|RandomFloatinRange (.x _changedirectionrange) (.y _changedirectionrange))))

(event EventReceiveTickAI
  (params (OwnerController :type AI%20Controller%20Object%20Reference) (ControlledPawn :type Pawn%20Object%20Reference) (DeltaSeconds :type Float%20%28single-precision%29))
  (bind _returnvalue (Transformation|GetActorLocation ControlledPawn))
  (bind _targetkey (Variables|Default|GetTargetKey))
  (bind _returnvalue_2 (AI|BehaviorTree|GetBlackboardValueasActor _targetkey))
  (Utilities|IsValid _returnvalue_2
    (:Is%20Valid
      (AI|SetFocus OwnerController _returnvalue_2)
      (AI|BehaviorTree|SetBlackboardValueasVector (Variables|Default|GetTargetLocation) (+ _returnvalue (* (Math|Vector|CrossProduct (Math|Vector|GetUnitDirection(Vector) _returnvalue (Transformation|GetActorLocation _returnvalue_2)) (Math|Vector|VectorUp)) (Variables|Default|GetDistance) (Math|Float|SelectFloat -1.0 1.0 (Variables|Default|GetFlipDirection))))))))

(event EventReceiveActivationAI
  (params (OwnerController :type AI%20Controller%20Object%20Reference) (ControlledPawn :type Pawn%20Object%20Reference))
  (bind _changedirectionrange (Variables|Default|GetChangeDirectionRange))
  (Variables|Default|SetFlipDirection (Math|Random|RandomBool))
  (if (Utilities|Operators|NotEqual(!=) :A (Variables|Default|GetChangeDirectionRange))
    (Utilities|Time|SetTimerbyEvent (delegate Custom|OnDirectionChange) (Math|Random|RandomFloatinRange (.x _changedirectionrange) (.y _changedirectionrange)))))