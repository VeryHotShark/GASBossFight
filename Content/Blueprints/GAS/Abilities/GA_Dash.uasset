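; Gameplay Ability for the player's dodge dash, committing first and blocking move input until it ends.
; With a lock target, it plays a Dodges montage picked by SelectDodgeMontage, scaling root motion by index, or a backward dodge when stationary.
; Without a target, it always plays the forward dodge.
; Montage blend-out or interruption ends the ability, restoring input and stopping montages; a root-motion force dash branch remains unconnected.
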(event Ability|EventActivateAbility
  (bind _returnvalue (Ability|GetActorInfo))
  (bind _returnvalue_2 (|SelectDodgeMontage (.avataractor _returnvalue)))
  (bind _returnvalue_3 (Ability|CommitAbility))
  (if _returnvalue_3
    (Input|SetIgnoreMoveInput (.playercontroller _returnvalue) true)
    (bind _asbp_player_character (Utilities|Casting|CastToBP_PlayerCharacter (.avataractor _returnvalue)))
    (Variables|/Game/Blueprints/Characters/BP_PlayerCharacter.BP_PlayerCharacter_C|GetLockTarget _asbp_player_character
      (:then
        (|PlayMontageandWaitProxy "None" (select (not (Math|Vector|VectorIsNearlyZero (Math|Vector|Normalize (Transformation|GetVelocity (.avataractor _returnvalue))))) (Utilities|Array|Get(acopy) (Variables|Default|GetDodges) _returnvalue_2) "/Game/Animations/Sword_Anim/Dodge/AM_Doge_Combat_B_Seq.AM_Doge_Combat_B_Seq") 1.2 "None" true (Math|Float|SelectFloat 1.2 0.7 (Utilities|Array|ContainsItem (Utilities|Array|MakeArray 1 3 5 7) _returnvalue_2)) 0.2
          (:OnBlendOut
            _)
          (:OnInterrupted
            _))
        (Ability|EndAbility))
      (:else
        (|PlayMontageandWaitProxy "None" "/Game/Animations/Sword_Anim/Dodge/AM_Doge_Combat_F_Seq.AM_Doge_Combat_F_Seq" 1.2 "None" true 1.0 0.2
          (:OnBlendOut
            _)
          (:OnInterrupted
            _))
        (Ability|EndAbility)))
    (else
      (Ability|CancelAbility))))

(event Ability|EventOnEndAbility
  (params (bWasCancelled :type Boolean))
  (bind _returnvalue (Ability|GetActorInfo))
  (Input|SetIgnoreMoveInput (.playercontroller _returnvalue) false)
  (Animation|Montage|MontageStop (Components|SkeletalMesh|GetAnimInstance (.skeletalmeshcomponent _returnvalue)) 0.0 0))