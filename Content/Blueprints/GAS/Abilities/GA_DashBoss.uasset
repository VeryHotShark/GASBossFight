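; GA_DashBoss is a Gameplay Ability that makes a boss perform a random dodge dash.
; After committing, it plays a random Dodges montage sped up from a slight start offset, scaling root motion up for two specific indices and down for others.
; The ability ends on blend out or interruption, or cancels if the commit fails.
; OnEndAbility stops montage playback on the owner's AnimInstance with zero blend-out time.
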(event Ability|EventActivateAbility
  (bind _dodges (Variables|Default|GetDodges))
  (bind _returnvalue (Ability|CommitAbility))
  (if _returnvalue
    (bind _output_get (Variables|Default|SetRandomInt (Math|Random|RandomIntegerinRange 0 (Utilities|Array|LastIndex _dodges))))
    (|PlayMontageandWaitProxy "None" (Utilities|Array|Get(acopy) _dodges _output_get) 1.2 "None" true (Math|Float|SelectFloat 1.2 0.7 (Utilities|Array|ContainsItem (Utilities|Array|MakeArray 1 3) (Variables|Default|GetRandomInt))) 0.2
      (:OnBlendOut
        _)
      (:OnInterrupted
        _))
    (Ability|EndAbility)
    (else
      (Ability|CancelAbility))))

(event Ability|EventOnEndAbility
  (params (bWasCancelled :type Boolean))
  (Animation|Montage|MontageStop (Components|SkeletalMesh|GetAnimInstance (.skeletalmeshcomponent (Ability|GetActorInfo))) 0.0 0))