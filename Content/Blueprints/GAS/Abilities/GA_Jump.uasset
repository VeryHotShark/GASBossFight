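; GA_Jump is a Gameplay Ability that makes the player character jump.
; Activation is allowed only when the avatar casts to XPlayerCharacter and CanJump returns true.
; On activation it prints a debug string and commits, then calls Jump on the owning BP_PlayerCharacter and applies GE_State_Jump to the owner.
; A failed commit cancels the ability, while the successful path never calls EndAbility.
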(event Ability|EventActivateAbility
  (Development|PrintString "JUMPo")
  (bind _returnvalue (Ability|CommitAbility))
  (if _returnvalue
    (bind _asbp_player_character (Utilities|Casting|CastToBP_PlayerCharacter (.OwnerActor (Utilities|Struct|BreakGameplayAbilityActorInfo (Ability|GetActorInfo)))))
    (Character|Jump _asbp_player_character)
    (Ability|ApplyGameplayEffectToOwner "/Game/Blueprints/GAS/Effects/GE_State_Jump.GE_State_Jump_C")
    (else
      (Ability|CancelAbility))))

(event Ability|EventOnEndAbility
  (params (bWasCancelled :type Boolean)))

(fn K2CanActivateAbility
  (params (ActorInfo :type Gameplay%20Ability%20Actor%20Info%20Structure) (Handle :type Gameplay%20Ability%20Spec%20Handle%20Structure))
  (bind _asxplayer_character (Utilities|Casting|CastToXPlayerCharacter (.AvatarActor (Utilities|Struct|BreakGameplayAbilityActorInfo ActorInfo)))
    (:then
      (return "" (Character|CanJump _asxplayer_character)))
    (:CastFailed
      (return "" false))))